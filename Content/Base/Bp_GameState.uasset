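; Game state Blueprint that runs a level's timer and completion check, judged by fire count.
; BeginPlay creates and shows the W_Game_Screen widget.
; Tick, throttled by a 0.1-second Delay, increments and prints Timer, then compares NumberOfFire with FireAchieved.
; On a match it prints a debug message and, once only, switches the widget's switcher page, waits three seconds and opens NextLevel.
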(event EventBeginPlay
  (bind _returnvalue (UserInterface|CreateWidget "/Game/A_PompierPomp/UI/W_Game_Screen.W_Game_Screen_C"))
  (Variables|Default|SetUI _returnvalue)
  (UserInterface|Viewport|AddtoViewport _returnvalue 0))

(event EventTick
  (params (DeltaSeconds :type Float%20%28single-precision%29))
  (Utilities|FlowControl|Delay 0.1)
  (Utilities|FlowControl|Sequence
    (:then_0
      (Variables|Default|SetTimer (+ (Variables|Default|GetTimer) 0.1))
      (Development|PrintString (Utilities|String|ToString(Float) (Variables|Default|GetTimer)) true true "(R=0.000000,G=0.660000,B=1.000000,A=1.000000)" 0.1))
    (:then_1
      (if (== (Variables|Default|GetNumberOfFire) (Variables|Default|GetFireAchieved))
        (Development|PrintString "levelDone!!!!!!!")
        (|DoOnceMultiInput
          (:A%20Out
            (Class|WidgetSwitcher|SetActiveWidgetIndex (Variables|/Game/A_PompierPomp/UI/W_Game_Screen.W_Game_Screen_C|GetWidgetSwitcher_39 (Variables|Default|GetUI)) 1)
            (Utilities|FlowControl|Delay 3.0)
            (Game|OpenLevel(byName) (Variables|Default|GetNextLevel))))))))

(fn ConstructionScript)
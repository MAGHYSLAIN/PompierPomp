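; Blueprint that cycles particle text through a list of names on a timer.
; On BeginPlay it starts a looping timer that fires every two seconds.
; Each tick increments an index and passes the next entry in the Names array, wrapping by modulo, to the ParticleTextParam component's SetParamText.
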(event Custom|Update%20Text
  (bind _result (Math|Integer|IncrementInt (Variables|Default|GetIndex))
    (:%20%20
      (Class|ParticleTextParamComponent|SetParamText (Variables|Default|GetParticleTextParam) (Utilities|Array|Get(acopy) (Variables|Default|GetNames) (Math|Integer|%(Integer) _result (Utilities|Array|Length (Variables|Default|GetNames))))))))

(event EventBeginPlay
  (Utilities|Time|SetTimerbyEvent (delegate Custom|Update%20Text) 2.0 true))

(fn ConstructionScript)
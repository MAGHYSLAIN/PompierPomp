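; Particle text effect actor that repeatedly spawns P_RATTA emitters around itself from BeginPlay.
; STARTFX calls SpawnPFX, then re-arms itself on a short randomized timer.
; SpawnPFX attaches each emitter to the root at a random point on an upper arc in the YZ plane, rolled by the arc angle.
; STOPFX clears a timer named "PEW", which matches no function here, rather than the STARTFX timer.
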(event Custom|STARTFX
  (Utilities|Time|ClearTimerbyFunctionName 0 "PEW")
  (CallFunction|SpawnPFX)
  (Utilities|Time|SetTimerbyEvent (delegate Custom|STARTFX) (Math|Random|RandomFloatinRange 0.3 0.6)))

(event Custom|STOPFX
  (Utilities|Time|ClearTimerbyFunctionName 0 "PEW"))

(event EventBeginPlay
  (CallFunction|STARTFX))

(fn ConstructionScript)

(fn SpawnPFX
  (bind _output_get (LocalVariables|SetNewLocalVar_0 (Math|Random|RandomFloatinRange -1.0 1.0)))
  (Effects|SpawnEmitterAttached "/Game/ParticleText/P_RATTA.P_RATTA" (Variables|Default|GetDefaultSceneRoot) "None" (* (Math|Vector|MakeVector 0.0 (Math|Trig|Sin(Radians) _output_get) (Math|Trig|Cos(Radians) _output_get)) (Math|Random|RandomFloatinRange 1e+01 18.0)) (Math|Rotator|MakeRotator (Math|Trig|RadiansToDegrees (LocalVariables|GetNewLocalVar_0)) 0.0 0.0)))
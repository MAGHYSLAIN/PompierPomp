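; Per-level game manager for PompierPomp that hands the level's settings to the game state and starts the audio.
; On BeginPlay it casts to Bp_GameState and copies in the timer, fire count, next level and level name from its own variables.
; If the cast succeeds, it then plays the intro sound and, after a fixed delay, starts the song as 2D audio.
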(event EventBeginPlay
  (bind _asbp_game_state (Utilities|Casting|CastToBp_GameState (Game|GetGameState)))
  (Variables|/Game/A_PompierPomp/Base/Bp_GameState.Bp_GameState_C|SetTimer _asbp_game_state (Variables|Default|GetTime))
  (Variables|/Game/A_PompierPomp/Base/Bp_GameState.Bp_GameState_C|SetNumberOfFire _asbp_game_state (Variables|Default|GetNumberOfFire))
  (Variables|/Game/A_PompierPomp/Base/Bp_GameState.Bp_GameState_C|SetNextLevel _asbp_game_state (Utilities|String|StringToName (Variables|Default|GetNextLevel)))
  (Variables|/Game/A_PompierPomp/Base/Bp_GameState.Bp_GameState_C|SetLevelName _asbp_game_state (Variables|Default|GetLevelName))
  (Audio|PlaySound2D "/Game/A_PompierPomp/Sound/Pompier_Intro.Pompier_Intro" 1.0 1.0 0.0 0 0)
  (Utilities|FlowControl|Delay 6.0)
  (Audio|PlaySound2D (Variables|Default|GetSong) 1.0 1.0 0.0 0 0))

(event Collision|EventActorBeginOverlap
  (params (OtherActor :type Actor%20Object%20Reference)))

(event EventTick
  (params (DeltaSeconds :type Float%20%28single-precision%29)))

(fn ConstructionScript)